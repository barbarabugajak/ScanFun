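; Player character for a scanning mechanic, with Enhanced Input movement, roll rotation and a score HUD.
; Movement sets actor location directly, without sweep, and IA_Scan activates GA_Scan through the Ability System Component.
; Ability and attribute events update the score, fade the scan indicator material, report failed activation and widen the beam via timelines.
; Debug keys switch scanner types looked up by name in ScannableManagementSubsystem, and a quit key serves build tests.
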(event `self.ReceiveBeginPlay`
  ; Bind Enhanced Input Mapping Context
  (bind _asplayer_controller (cast `PlayerController` (`self.GetController`)))
  (`EnhancedInputSubsystemInterface.AddMappingContext` (pcsubsystem `EnhancedInputLocalPlayerSubsystem` _asplayer_controller) "/Game/Input/IMC_Default.IMC_Default" 0 (struct))
  ; Add UI
  (bind _returnvalue (`|CreateWidget` "/Game/UI/WBP_HUD.WBP_HUD_C"))
  (bind _output_get (set `self.HUD` _returnvalue))
  (`UserWidget.AddToViewport` _output_get 0))

(event `EnhancedInput|/Game/Input/IA_Move`
  (params (ActionValue :type "Vector Structure") (ElapsedSeconds :type "Float (double-precision)") (TriggeredSeconds :type "Float (double-precision)") (InputAction :type "InputAction Object Reference" :default "/Game/Input/IA_Move.IA_Move"))
  ; Movement
  (:`Triggered`
    (`self.K2_SetActorLocation` (+ (* ActionValue (`self.MovementSpeed`) (`GameplayStatics.GetWorldDeltaSeconds`)) (`self.K2_GetActorLocation`)))))

(event `self.AttributeSet_ScoreChaned`
  (params (OldValue :type "Float (single-precision)") (NewValue :type "Float (single-precision)"))
  (bind _hud (`self.HUD`))
  ; Change value of score in UI
  (`/Engine/EditorBlueprintResources/StandardMacros.IsValid` _hud
    (:`Is Valid`
      (`/Game/UI/WBP_Score.ScoreValueChanged` (`/Game/UI/WBP_HUD.WBP_Score` _hud) (`KismetTextLibrary.Conv_DoubleToText` NewValue "HalfToEven" false true 1 324 2 2)))))

(event `EnhancedInput|/Game/Input/IA_Scan`
  (params (ActionValue :type Boolean) (ElapsedSeconds :type "Float (double-precision)") (TriggeredSeconds :type "Float (double-precision)") (InputAction :type "InputAction Object Reference" :default "/Game/Input/IA_Scan.IA_Scan"))
  ; Activate Scan Ability
  (:`Started`
    (`AbilitySystemComponent.TryActivateAbilityByClass` (`self.ASC`) "/Game/Blueprints/GAS/Abilities/GA_Scan.GA_Scan_C" true)))

(event `self.ScanAbility_Activated`
  (params (didAnythingGetScanned :type Boolean))
  ; Scan Visual Indicator
  (bind _returnvalue (`MaterialInstanceDynamic.K2_GetScalarParameterValue` (`self.DynMaterial`) "Opacity"))
  (bind (_direction _opacity) (`Timeline|ScanIndicator` :!via `PlayFromStart`)
    (:`Update`
      (`MaterialInstanceDynamic.SetScalarParameterValue` (`self.DynMaterial`) "Opacity" (* _returnvalue _opacity)))))

(event `EnhancedInput|/Game/Input/IA_Rotate`
  (params (ActionValue :type "Float (double-precision)") (ElapsedSeconds :type "Float (double-precision)") (TriggeredSeconds :type "Float (double-precision)") (InputAction :type "InputAction Object Reference" :default "/Game/Input/IA_Rotate.IA_Rotate"))
  (bind (_returnvalue_roll _returnvalue_pitch _returnvalue_yaw) (`KismetMathLibrary.BreakRotator` (`self.K2_GetActorRotation`)))
  ; Rotation
  (:`Triggered`
    (`self.K2_SetActorRelativeRotation` (`KismetMathLibrary.MakeRotator` (+ (* ActionValue (`self.RotationSpeed`) (`GameplayStatics.GetWorldDeltaSeconds`)) _returnvalue_roll) _returnvalue_pitch _returnvalue_yaw))))

(event `self.ScanAbility_ActivationFailed`
  (`KismetSystemLibrary.PrintString` "Ability in Cooldown" true true (struct :`R` 1.0 :`G` 0.031268 :`A` 1.0)))

(event `EnhancedInput|/Game/Input/IA_Quit`
  (params (ActionValue :type Boolean) (ElapsedSeconds :type "Float (double-precision)") (TriggeredSeconds :type "Float (double-precision)") (InputAction :type "InputAction Object Reference" :default "/Game/Input/IA_Quit.IA_Quit"))
  ; Quit on esc (For Build Tests)
  (:`Started`
    (`KismetSystemLibrary.QuitGame` null "Quit")))

(event `EnhancedInput|/Game/Input/IA_1`
  (params (ActionValue :type Boolean) (ElapsedSeconds :type "Float (double-precision)") (TriggeredSeconds :type "Float (double-precision)") (InputAction :type "InputAction Object Reference" :default "/Game/Input/IA_1.IA_1"))
  ; (Debug) Testing Scanner switching
  (:`Triggered`
    (bind _returnvalue (`ScannableManagementSubsystem.GetScannerTypeFromName` (subsystem `ScannableManagementSubsystem`) "Classic"))
    (`self.SetupScannerBeamParams` _returnvalue)))

(event `EnhancedInput|/Game/Input/IA_2`
  (params (ActionValue :type Boolean) (ElapsedSeconds :type "Float (double-precision)") (TriggeredSeconds :type "Float (double-precision)") (InputAction :type "InputAction Object Reference" :default "/Game/Input/IA_2.IA_2"))
  ; (Debug) Testing Scanner switching
  (:`Triggered`
    (bind _returnvalue (`ScannableManagementSubsystem.GetScannerTypeFromName` (subsystem `ScannableManagementSubsystem`) "TestCube"))
    (`self.SetupScannerBeamParams` _returnvalue)))

(event `EnhancedInput|/Game/Input/IA_3`
  (params (ActionValue :type Boolean) (ElapsedSeconds :type "Float (double-precision)") (TriggeredSeconds :type "Float (double-precision)") (InputAction :type "InputAction Object Reference" :default "/Game/Input/IA_3.IA_3"))
  ; (Debug) Testing Scanner switching
  (:`Triggered`
    (bind _returnvalue (`ScannableManagementSubsystem.GetScannerTypeFromName` (subsystem `ScannableManagementSubsystem`) "PurpleCone"))
    (`self.SetupScannerBeamParams` _returnvalue)))

(event `EnhancedInput|/Game/Input/IA_4`
  (params (ActionValue :type Boolean) (ElapsedSeconds :type "Float (double-precision)") (TriggeredSeconds :type "Float (double-precision)") (InputAction :type "InputAction Object Reference" :default "/Game/Input/IA_4.IA_4"))
  ; (Debug) Testing Scanner switching
  (:`Triggered`
    (bind _returnvalue (`ScannableManagementSubsystem.GetScannerTypeFromName` (subsystem `ScannableManagementSubsystem`) "BlueCone"))
    (`self.SetupScannerBeamParams` _returnvalue)))

(event `self.ScanAbility_WidenBeam`
  (params (oldWidth :type "Float (single-precision)") (newWidth :type "Float (single-precision)"))
  (bind (_direction _value) (`Timeline|Timeline` :!via `PlayFromStart`)
    (:`Update`
      (set `self.currentBeamWidthCoefficient` (`KismetMathLibrary.Lerp` oldWidth newWidth _value)))))

(fn `UserConstructionScript`)