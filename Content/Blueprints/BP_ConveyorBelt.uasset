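; BP_ConveyorBelt is a conveyor belt actor that serves as the spawn location for scannable items.
; On BeginPlay it registers itself as the belt with the ScannableManagementSubsystem and hands over a spawn point.
; GetScannableSpawnPoint derives that point from the actor location, offset along world Y and Z by the extents of its colliding bounds.
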(event `self.ReceiveBeginPlay`
  (bind _returnvalue (subsystem `ScannableManagementSubsystem`))
  (bind _spawn_point (`self.GetScannableSpawnPoint`))
  (set `ScannableManagementSubsystem.SpawnLocation` _spawn_point _returnvalue)
  (set `ScannableManagementSubsystem.Belt` self _returnvalue))

(fn `GetScannableSpawnPoint`
  (returns (`Spawn Point` :type "Vector Structure"))
  (bind (_origin _boxextent) (`self.GetActorBounds` true))
  (return (+ (`self.K2_GetActorLocation`) (`KismetMathLibrary.MakeVector` 0.0 (.y _boxextent) (.z _boxextent)))))

(fn `UserConstructionScript`)